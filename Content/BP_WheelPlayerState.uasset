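; Player state for a wheel word-puzzle game (Grump of Fortune) that manages score banking and CPU difficulty selection.
; BankCurrentScore adds the current round score to the banked score, then resets the round score.
; SetCPUDifficulty writes the chosen difficulty to the game mode, along with preset tuning for CPU letter-guessing skill, solve threshold and incorrect-solve chance.
; The event graph and construction script are empty.
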(event EventBeginPlay)

(event EventTick
  (params (DeltaSeconds :type Float%20%28single-precision%29)))

(fn ConstructionScript)

(fn BankCurrentScore
  (Variables|Default|SetBankScore (+ (Variables|Default|GetBankScore) (Variables|Default|GetCurrentRoundScore)))
  (Variables|Default|SetCurrentRoundScore 0))

(fn SetCPUDifficulty
  (params (Difficulty :type E_CPUDifficulty%20Enum :default "NewEnumerator0"))
  (bind _asgm_grump_of_fortune (Utilities|Casting|CastToGM_GrumpOfFortune (Game|GetGameMode)))
  (bind _output_get (Variables|/Game/Blueprints/GM_GrumpOfFortune.GM_GrumpOfFortune_C|SetCPUDifficulty _asgm_grump_of_fortune Difficulty))
  (switch Utilities|FlowControl|Switch|SwitchonE_CPUDifficulty _output_get
    (:NewEnumerator0
      (Variables|/Game/Blueprints/GM_GrumpOfFortune.GM_GrumpOfFortune_C|SetLetterGuessingSkill _asgm_grump_of_fortune 0.3)
      (Variables|/Game/Blueprints/GM_GrumpOfFortune.GM_GrumpOfFortune_C|SetSolveThreshold _asgm_grump_of_fortune 0.8)
      (Variables|/Game/Blueprints/GM_GrumpOfFortune.GM_GrumpOfFortune_C|SetIncorrectSolveChance _asgm_grump_of_fortune 0.4))
    (:NewEnumerator1
      (Variables|/Game/Blueprints/GM_GrumpOfFortune.GM_GrumpOfFortune_C|SetLetterGuessingSkill _asgm_grump_of_fortune 0.6)
      (Variables|/Game/Blueprints/GM_GrumpOfFortune.GM_GrumpOfFortune_C|SetSolveThreshold _asgm_grump_of_fortune 0.65)
      (Variables|/Game/Blueprints/GM_GrumpOfFortune.GM_GrumpOfFortune_C|SetIncorrectSolveChance _asgm_grump_of_fortune 0.2))
    (:NewEnumerator2
      (Variables|/Game/Blueprints/GM_GrumpOfFortune.GM_GrumpOfFortune_C|SetLetterGuessingSkill _asgm_grump_of_fortune 0.85)
      (Variables|/Game/Blueprints/GM_GrumpOfFortune.GM_GrumpOfFortune_C|SetSolveThreshold _asgm_grump_of_fortune 0.45)
      (Variables|/Game/Blueprints/GM_GrumpOfFortune.GM_GrumpOfFortune_C|SetIncorrectSolveChance _asgm_grump_of_fortune 0.05))))