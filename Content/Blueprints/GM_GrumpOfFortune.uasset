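; Game manager for a Wheel of Fortune-style word puzzle game, running human and CPU players through rounds to a highest-bank winner.
; It spawns a puzzle manager and player states, then picks a random puzzle each round.
; GuessLetter reveals board letters, scores hits, completes solved rounds or passes the turn on misses, with dispatchers announcing events.
; CPU play is unfinished: turns only print a placeholder, and ExecuteCPUTurn always returns before its solve-or-guess logic.
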(event EventBeginPlay
  (bind _returnvalue (Game|SpawnActorfromClass "/Game/BP_PuzzleManager.BP_PuzzleManager_C" (Math|Transform|MakeTransform "0, 0, 0" "0, 0, 0" "1.000000,1.000000,1.000000") "Undefined" "MultiplyWithRoot" 0 0 0))
  (Variables|Default|SetPuzzleManager _returnvalue))

(event EventTick
  (params (DeltaSeconds :type Float%20%28single-precision%29)))

(fn ConstructionScript)

(fn InitializeGame
  (params (NumberOfHumans :type Integer) (NumberOfBots :type Integer))
  (Variables|Default|SetHumanPlayerCount NumberOfHumans)
  (Variables|Default|SetCPUPlayerCount NumberOfBots)
  (CallFunction|RegisterPlayers)
  (Variables|Default|SetCurrentRound 1)
  (Variables|Default|SetGamePhase "NewEnumerator0"))

(fn RegisterPlayers
  (Utilities|Array|Clear (Variables|Default|GetPlayerArray))
  ;[0.158 0 0 0.5] Set Human Players
  (for _index (range 0 (- (Variables|Default|GetHumanPlayerCount) 1))
    (bind _returnvalue (Game|SpawnActorfromClass "/Game/BP_WheelPlayerState.BP_WheelPlayerState_C" (Math|Transform|MakeTransform "0, 0, 0" "0, 0, 0" "1.000000,1.000000,1.000000") "Undefined" "MultiplyWithRoot" 0 0))
    (Variables|/Game/BP_WheelPlayerState.BP_WheelPlayerState_C|SetPlayerName _returnvalue (Utilities|GetDisplayName _returnvalue))
    (Variables|/Game/BP_WheelPlayerState.BP_WheelPlayerState_C|SetIsAIControlled _returnvalue false)
    (Variables|/Game/BP_WheelPlayerState.BP_WheelPlayerState_C|SetCurrentRoundScore _returnvalue 0)
    (Variables|/Game/BP_WheelPlayerState.BP_WheelPlayerState_C|SetBankScore _returnvalue 0)
    (Utilities|Array|Add (Variables|Default|GetPlayerArray) _returnvalue)
    (switch int (LocalVariables|GetDifficultyIndex)
      (:0
        (Variables|Default|SetCPUDifficulty "NewEnumerator0"))
      (:1
        (Variables|Default|SetCPUDifficulty "NewEnumerator1"))
      (:2
        (Variables|Default|SetCPUDifficulty "NewEnumerator2")))
    (bind _result (Math|Integer|IncrementInt (LocalVariables|GetDifficultyIndex))
      (:%20%20
        (if (> _result 2)
          (LocalVariables|SetDifficultyIndex 0)))))
  ;[0 0.412 0.6476 0.5] Set CPU Players
  (for _index_2 (range 0 (- (Variables|Default|GetCPUPlayerCount) 1))
    (bind _returnvalue_2 (Game|SpawnActorfromClass "/Game/BP_WheelPlayerState.BP_WheelPlayerState_C" (Math|Transform|MakeTransform "0, 0, 0" "0, 0, 0" "1.000000,1.000000,1.000000") "Undefined" "MultiplyWithRoot" 0 0))
    (Variables|/Game/BP_WheelPlayerState.BP_WheelPlayerState_C|SetPlayerName _returnvalue_2 (Utilities|GetDisplayName _returnvalue_2))
    (Variables|/Game/BP_WheelPlayerState.BP_WheelPlayerState_C|SetIsAIControlled _returnvalue_2 true)
    (Variables|/Game/BP_WheelPlayerState.BP_WheelPlayerState_C|SetCurrentRoundScore _returnvalue_2 0)
    (Variables|/Game/BP_WheelPlayerState.BP_WheelPlayerState_C|SetBankScore _returnvalue_2 0)
    (Utilities|Array|Add (Variables|Default|GetPlayerArray) _returnvalue_2))
  (Variables|Default|SetCurrentPlayerIndex 0)
  (Development|PrintString (Utilities|String|ToString(Text) (Utilities|Text|FormatText "Human players: {0} 
CPU players: {1}" (Variables|Default|GetHumanPlayerCount) (Variables|Default|GetCPUPlayerCount))) true true "(R=1.000000,G=0.000000,B=0.179450,A=1.000000)" 5.0))

(fn SetupRound
  (bind _puzzlestruct (Default|SelectRandomPuzzle (Variables|Default|GetPuzzleManager)))
  (Variables|Default|SetCurrentPuzzle _puzzlestruct)
  (bind _array_element (Utilities|Array|ForEachLoopwithBreak (Variables|Default|GetPlayerArray))
    (:LoopBody
      (bind _asbp_wheel_player_state (Utilities|Casting|CastToBP_WheelPlayerState _array_element)
        (:then
          (Variables|/Game/BP_WheelPlayerState.BP_WheelPlayerState_C|SetCurrentRoundScore _asbp_wheel_player_state 0)
          (Variables|/Game/BP_WheelPlayerState.BP_WheelPlayerState_C|SetPlayerTurn _asbp_wheel_player_state false)
          (Variables|/Game/BP_WheelPlayerState.BP_WheelPlayerState_C|SetCurrentRoundScore _asbp_wheel_player_state 0))
        (:CastFailed
          (Development|PrintString "Unexpected Player Type in Player Array"))))
    (:Completed
      (Variables|Default|SetGamePhase "NewEnumerator1")
      (Variables|Default|SetCurrentPlayerIndex 0) ; Change to ensure winner of previous round goes first
      (bind _result (Math|Integer|IncrementInt (Variables|Default|GetCurrentRound))
        (:%20%20
          (Variables|Default|SetCurrentRound _result)
          (Development|PrintString (Utilities|String|ToString(Text) (Utilities|Text|FormatText "Round {0} Started! 
Category: {1} 
Phase: {2}" (Variables|Default|GetCurrentRound) (.Category (Utilities|Struct|BreakS_PuzzleData (Variables|Default|GetCurrentPuzzle))) (.Phrase (Utilities|Struct|BreakS_PuzzleData (Variables|Default|GetCurrentPuzzle))))) true true "(R=0.000000,G=1.000000,B=0.044649,A=1.000000)" 5.0)
          (Default|CallOnRoundSetup))))))

(fn NextPlayerTurn
  (bind _result (Math|Integer|IncrementInt (Variables|Default|GetCurrentPlayerIndex))
    (:%20%20
      (if (< (Utilities|Array|Length (Variables|Default|GetPlayerArray)) _result)
        (bind _output_get (Variables|Default|SetCurrentPlayerIndex _result))
        (bind _asbp_wheel_player_state (Utilities|Casting|CastToBP_WheelPlayerState (Utilities|Array|Get(acopy) (Variables|Default|GetPlayerArray) _output_get)))
        (if (Variables|/Game/BP_WheelPlayerState.BP_WheelPlayerState_C|GetIsAIControlled _asbp_wheel_player_state)
          ;[1 0 0 0.5 22] NEED TO WRITE ExecuteCPUTurn FUNCTION
          (Development|PrintString "Call ExecuteCPUTurn" :!label _label)
          (else
            (Default|CallOnPlayerTurnBegin :!label _label_2)))
        (else
          (bind _output_get_2 (Variables|Default|SetCurrentPlayerIndex 0))
          (bind _asbp_wheel_player_state_2 (Utilities|Casting|CastToBP_WheelPlayerState (Utilities|Array|Get(acopy) (Variables|Default|GetPlayerArray) _output_get_2)))
          (if (Variables|/Game/BP_WheelPlayerState.BP_WheelPlayerState_C|GetIsAIControlled _asbp_wheel_player_state_2)
            (goto _label)
            (else
              (goto _label_2))))))))

(fn CompleteRound
  (params (WinningPlayerIndex :type Integer))
  (bind _returnvalue (Actor|GetActorOfClass "/Game/BP_WheelPlayerState.BP_WheelPlayerState_C"))
  (Default|BankCurrentScore _returnvalue)
  (Variables|Default|SetGamePhase "NewEnumerator2")
  (bind _result (Math|Integer|IncrementInt (Variables|Default|GetCurrentRound))
    (:%20%20
      (bind _output_get (Variables|Default|SetCurrentRound _result))
      (if (> _output_get (Variables|Default|GetRoundsPerGame))
        (CallFunction|EndGame)
        (else
          (Utilities|Time|SetTimerbyFunctionName 0 "StartNextRound" 3.0)
          (CallFunction|SetupRound)
          (Default|CallOnRoundComplete WinningPlayerIndex))))))

(fn StartNextRound
  (CallFunction|SetupRound))

(fn EndGame
  (Variables|Default|SetGamePhase "NewEnumerator3")
  (for (_array_element _array_index) (Variables|Default|GetPlayerArray)
    (bind _asbp_wheel_player_state (Utilities|Casting|CastToBP_WheelPlayerState _array_element))
    (if (> (Variables|/Game/BP_WheelPlayerState.BP_WheelPlayerState_C|GetBankScore _asbp_wheel_player_state) (LocalVariables|GetHighestScore))
      (LocalVariables|SetHighestScore (Variables|/Game/BP_WheelPlayerState.BP_WheelPlayerState_C|GetBankScore _asbp_wheel_player_state))
      (LocalVariables|SetWinnerIndex _array_index)))
  (Development|PrintString (Utilities|String|ToString(Text) (Utilities|Text|FormatText "Game Over! Player {0} Wins with {1} points!" (LocalVariables|GetWinnerIndex) (LocalVariables|GetHighestScore)))))

(fn ExecuteCPUTurn
  (params (IndexOfCPU :type Integer))
  (bind _availableletters (LocalVariables|GetAvailableLetters))
  (bind _availableletters_2 (LocalVariables|GetAvailableLetters))
  (bind _puzzleboard (Variables|Default|GetPuzzleBoard))
  (Utilities|Casting|CastToBP_WheelPlayerState (Utilities|Array|Get(acopy) (Variables|Default|GetPlayerArray) IndexOfCPU))
  (bind _issolved (Default|IsPuzzleSolved _puzzleboard))
  (LocalVariables|SetIsCurrentPuzzleSolved _issolved)
  (if true
    (return)
    (else
      (bind _percentage (Default|GetRevealPercentage _puzzleboard))
      (if (>= _percentage (Variables|Default|GetSolveThreshold))
        (if (> (Math|Random|RandomFloatinRange 0.0 1.0) (Variables|Default|GetIncorrectSolveChance))
          (CallFunction|CompleteRound IndexOfCPU)
          (else
            (CallFunction|NextPlayerTurn)
            (for _index (range (Utilities|Array|LastIndex _availableletters) 0)
              (if (Utilities|Array|ContainsItem (Variables|Default|GetUsedLetters) (Utilities|Array|Get(acopy) _availableletters _index))
                (Utilities|Array|RemoveIndex (LocalVariables|GetAvailableLetters) _index)
                (if (<= (Math|Random|RandomFloatinRange 0.0 1.0) (Variables|Default|GetLetterGuessingSkill))
                  (LocalVariables|SetSelectedLetter (Utilities|Array|Get(acopy) (LocalVariables|GetAvailableLetters)))
                  (else
                    (LocalVariables|SetSelectedLetter (Utilities|Array|Get(acopy) _availableletters_2 (Math|Random|RandomIntegerinRange 0 (- (Utilities|Array|Length _availableletters_2) 1))))))
                (Development|PrintString (Utilities|String|ToString(Text) (Utilities|Text|FormatText "CPU Selected Letter: {SelectedLetter}" (LocalVariables|GetSelectedLetter))))
                (Utilities|Array|Add (Variables|Default|GetUsedLetters) (LocalVariables|GetSelectedLetter))))))))))

(fn GuessLetter
  (params (Letter :type String) (PlayerIndex :type Integer))
  (Utilities|Array|Add (Variables|Default|GetUsedLetters) Letter)
  (bind _instancesrevealed (Default|RevealLetter (Variables|Default|GetPuzzleBoard) Letter))
  (bind _output_get (Variables|Default|SetInstancesRevealed _instancesrevealed))
  (if (> _output_get 0)
    (bind _asbp_wheel_player_state (Utilities|Casting|CastToBP_WheelPlayerState (Utilities|Array|Get(acopy) (Variables|Default|GetPlayerArray) PlayerIndex)))
    (Variables|/Game/BP_WheelPlayerState.BP_WheelPlayerState_C|SetCurrentRoundScore _asbp_wheel_player_state (* (Variables|Default|GetInstancesRevealed) (Variables|Default|GetLetterValue)))
    (Default|CallOnLetterGuessed Letter (Variables|Default|GetInstancesRevealed) PlayerIndex)
    (bind _issolved (Default|IsPuzzleSolved (Variables|Default|GetPuzzleBoard)))
    (if _issolved
      (CallFunction|CompleteRound PlayerIndex)
      (else
        (Development|PrintString "Allow Player to Spin Again Or whatever")))
    (else
      (Development|PrintString (Utilities|String|ToString(Text) (Utilities|Text|FormatText "There are no {Letter}'s" Letter)))
      (CallFunction|NextPlayerTurn))))